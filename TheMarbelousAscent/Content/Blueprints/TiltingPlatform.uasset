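; Platform that tilts toward the Player_Marble while the marble rests on it, then levels out once contact ends.
; Hit events flag contact, and the actor Hit also resets a timer that Tick uses to bridge brief gaps.
; Tick scales the normalized marble-to-platform offset into clamped pitch and roll, eased with RInterpTo.
; After HitResetTime without contact, the mesh returns to level at half the tilt speed.
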(event `self.PlatformMesh.OnComponentHit`
  (params (HitComponent :type "PrimitiveComponent Object Reference") (OtherActor :type "Actor Object Reference") (OtherComp :type "PrimitiveComponent Object Reference") (NormalImpulse :type "Vector Structure") (Hit :type "HitResult Structure (by ref)"))
  (cast `/Game/Blueprints/Player_Marble` OtherActor)
  (set `self.PlayerOnPlatform` true))

(event `self.ReceiveBeginPlay`
  (bind _asplayer_marble (cast `/Game/Blueprints/Player_Marble` (`GameplayStatics.GetPlayerPawn` 0)))
  (set `self.PlayerRef` _asplayer_marble))

(event `self.ReceiveTick`
  (params (DeltaSeconds :type "Float (single-precision)"))
  (bind _platformmesh (`self.PlatformMesh`))
  (bind _playerref (`self.PlayerRef`))
  (bind _platformmesh_2 (`self.PlatformMesh`))
  (bind _maxtiltangle (`self.MaxTiltAngle`))
  (bind _returnvalue (* (`self.MaxTiltAngle`) -1.0))
  (`/Engine/EditorBlueprintResources/StandardMacros.IsValid` _playerref
    (:`Is Valid`
      (set `self.TimeSinceHit` (+ (`self.TimeSinceHit`) (`GameplayStatics.GetWorldDeltaSeconds`)))
      (if (`self.PlayerOnPlatform`)
        (if (not (>= (`self.TimeSinceHit`) 0.1))
          (set `self.PlayerOnPlatform` false))
        (`SceneComponent.K2_SetRelativeRotation` _platformmesh (`KismetMathLibrary.RInterpTo` (`SceneComponent.RelativeRotation` _platformmesh) (`KismetMathLibrary.MakeRotator` (`KismetMathLibrary.FClamp` (* (.y (`KismetMathLibrary.Normal` (- (`SceneComponent.K2_GetComponentLocation` (`/Game/Blueprints/Player_Marble.Marble` _playerref)) (`SceneComponent.K2_GetComponentLocation` (`self.PlatformMesh`))))) (`self.TiltStrength`)) _returnvalue _maxtiltangle) (* (`KismetMathLibrary.FClamp` (* (.x (`KismetMathLibrary.Normal` (- (`SceneComponent.K2_GetComponentLocation` (`/Game/Blueprints/Player_Marble.Marble` _playerref)) (`SceneComponent.K2_GetComponentLocation` (`self.PlatformMesh`))))) (`self.TiltStrength`)) _returnvalue _maxtiltangle) -1.0)) (`GameplayStatics.GetWorldDeltaSeconds`) (`self.TiltSpeed`)) false false :!label _label)
        (elif (> (`self.TimeSinceHit`) (`self.HitResetTime`))
          (`SceneComponent.K2_SetRelativeRotation` _platformmesh_2 (`KismetMathLibrary.RInterpTo` (`SceneComponent.RelativeRotation` _platformmesh_2) (struct) (`GameplayStatics.GetWorldDeltaSeconds`) (/ (`self.TiltSpeed`) 2.0)) false false)
          (elif (<= (`self.TimeSinceHit`) 0.3)
            (goto _label)))))))

(event `self.ReceiveHit`
  (params (MyComp :type "PrimitiveComponent Object Reference") (Other :type "Actor Object Reference") (OtherComp :type "PrimitiveComponent Object Reference") (bSelfMoved :type Boolean) (HitLocation :type "Vector Structure") (HitNormal :type "Vector Structure") (NormalImpulse :type "Vector Structure") (Hit :type "HitResult Structure (by ref)"))
  (if (== Other (`self.PlayerRef`))
    (set `self.TimeSinceHit` 0.0)
    (set `self.PlayerOnPlatform` true)))

(fn `UserConstructionScript`)
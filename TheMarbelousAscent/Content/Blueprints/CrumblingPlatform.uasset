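; Crumbling platform actor that shakes when hit, breaks apart, then restores itself.
; A hit on the static platform starts a timeline that offsets it along X, guarded by IsShaking against retriggers.
; After WaitTime, FracturePlatform swaps the platform for a physics-simulated Geometry Collection by toggling visibility and collision.
; A fixed delay later, it resets the rest collection, hides it via DisableCrumble, and re-enables the intact platform.
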(event `self.ReceiveBeginPlay`
  (bind _returnvalue_location (`KismetMathLibrary.BreakTransform` (`SceneComponent.GetRelativeTransform` (`self.Crumbling_platformB`))))
  (set `self.StartLocation` _returnvalue_location)
  (`self.DisableCrumble`))

(event `self.ReceiveActorBeginOverlap`
  (params (OtherActor :type "Actor Object Reference")))

(event `self.Crumbling_platformB.OnComponentHit`
  (params (HitComponent :type "PrimitiveComponent Object Reference") (OtherActor :type "Actor Object Reference") (OtherComp :type "PrimitiveComponent Object Reference") (NormalImpulse :type "Vector Structure") (Hit :type "HitResult Structure (by ref)"))
  (if (not (`self.bIsShaking`))
    (set `self.bIsShaking` true)
    (bind (_direction _newtrack_0) (`Timeline|ShakingTimeline` :!via `PlayFromStart`)
      (:`Update`
        (`SceneComponent.K2_SetRelativeLocation` (`self.Crumbling_platformB`) (+ (`KismetMathLibrary.VLerp` (0.0 0.0 0.0) (15.0 0.0 0.0) _newtrack_0) (`self.StartLocation`)) false false)
        (`KismetSystemLibrary.Delay` (`self.WaitTime`))
        (set `self.bIsShaking` false)
        (`self.FracturePlatform`)
        (`KismetSystemLibrary.Delay` 10.0)
        (`GeometryCollectionComponent.SetRestCollection` (`self.GC_CrumblingPlatform`) "/Game/Fractures/GC_CrumblingPlatform.GC_CrumblingPlatform" true)
        (`self.DisableCrumble`)
        (`SceneComponent.SetVisibility` (`self.Crumbling_platformB`) true false)
        (`SceneComponent.SetHiddenInGame` (`self.Crumbling_platformB`) false false)
        (`PrimitiveComponent.SetCollisionEnabled` (`self.Crumbling_platformB`) "QueryAndPhysics")))))

(fn `DisableCrumble`
  (`PrimitiveComponent.SetSimulatePhysics` (`self.GC_CrumblingPlatform`) false)
  (`SceneComponent.SetVisibility` (`self.GC_CrumblingPlatform`) false false)
  (`SceneComponent.SetHiddenInGame` (`self.GC_CrumblingPlatform`) true false)
  (`PrimitiveComponent.SetCollisionEnabled` (`self.GC_CrumblingPlatform`) "NoCollision"))

(fn `FracturePlatform`
  (`SceneComponent.SetVisibility` (`self.Crumbling_platformB`) false false)
  (`SceneComponent.SetHiddenInGame` (`self.Crumbling_platformB`) true false)
  (`PrimitiveComponent.SetCollisionEnabled` (`self.Crumbling_platformB`) "NoCollision")
  (`PrimitiveComponent.SetSimulatePhysics` (`self.GC_CrumblingPlatform`) true)
  (`SceneComponent.SetVisibility` (`self.GC_CrumblingPlatform`) true false)
  (`SceneComponent.SetHiddenInGame` (`self.GC_CrumblingPlatform`) false false)
  (`PrimitiveComponent.SetCollisionEnabled` (`self.GC_CrumblingPlatform`) "QueryAndPhysics"))

(fn `UserConstructionScript`)
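; Moving platform actor that travels through a looping list of waypoints, pausing at each one.
; Each Tick while not waiting, StartMove steps toward the current world-space PosList entry at constant Speed, without sweep, and snaps onto it when within one step.
; On arrival, it sets Waiting and calls an event that delays by WaitTime, advances Index with modulo wrap, then resumes movement.
; BeginPlay stores StartLocation, which the movement logic never reads.
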(event `self.ReceiveBeginPlay`
  (set `self.StartLocation` (`self.K2_GetActorLocation`))
  (set `self.Index_0` 0))

(event `self.ReceiveTick`
  (params (DeltaSeconds :type "Float (single-precision)"))
  (if (not (`self.bWaiting`))
    (`self.StartMove` DeltaSeconds)))

(event `AdvanceWaypointAfterWait`
  (`KismetSystemLibrary.Delay` (`self.WaitTime`))
  (set `self.Index` (mod (+ (`self.Index`) 1) (`KismetArrayLibrary.Array_Length` (`self.posList`))))
  (set `self.bWaiting` false))

(fn `StartMove`
  (params (DeltaTime :type "Float (double-precision)"))
  (locals (NewLocalVar :type Integer :default 0))
  (if (== (`KismetArrayLibrary.Array_Length` (`self.posList`)) 0)
    (return)
    (else
      (set `self.TargetLocation` (`|GetArrayItem` (`self.posList`) (`self.Index`)))
      (bind _output_get (set `self.ToTarget` (- (`self.TargetLocation`) (`self.K2_GetActorLocation`))))
      (set `self.Distance` (`KismetMathLibrary.VSize` _output_get))
      (set `self.Step` (* (`self.speed`) DeltaTime))
      (if (<= (`self.Distance`) (`self.Step`))
        (`self.K2_SetActorLocation` (`self.TargetLocation`))
        (set `self.bWaiting` true)
        (`self.AdvanceWaypointAfterWait`)
        (return)
        (else
          (bind _output_get_2 (set `self.NewLocation` (+ (`self.K2_GetActorLocation`) (* (`KismetMathLibrary.Normal` (`self.ToTarget`)) (`self.Step`)))))
          (`self.K2_SetActorLocation` _output_get_2)
          (return))))))

(fn `UserConstructionScript`)
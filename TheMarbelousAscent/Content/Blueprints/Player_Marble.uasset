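; Player-controlled physics marble that rolls, brakes and jumps using Enhanced Input.
; Movement adds camera-relative forces, plus an opposing horizontal force once speed exceeds the maximum.
; A sphere trace with a slope check gates jumping and braking; jumps reset vertical velocity before the impulse, while braking progressively raises linear damping.
; Logic to halve movement force in the air exists but is never executed.
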(event `self.ReceiveBeginPlay`
  (bind _asplayer_controller (cast `PlayerController` (`self.GetController`)))
  (bind _returnvalue (pcsubsystem `EnhancedInputLocalPlayerSubsystem` _asplayer_controller))
  (`/Engine/EditorBlueprintResources/StandardMacros.IsValid` _returnvalue
    (:`Is Valid`
      (`EnhancedInputSubsystemInterface.AddMappingContext` _returnvalue "/Game/Input/Maps/playerMap.playerMap" 0 (struct)))))

(event `EnhancedInput|/Game/Input/Actions/PlayerActions/Left-Right_Action`
  (params (ActionValue :type "Float (double-precision)") (ElapsedSeconds :type "Float (double-precision)") (TriggeredSeconds :type "Float (double-precision)") (InputAction :type "InputAction Object Reference" :default "/Game/Input/Actions/PlayerActions/Left-Right_Action.Left-Right_Action"))
  (bind (_returnvalue_x _returnvalue_y _returnvalue_z) (`KismetMathLibrary.BreakVector` (`SceneComponent.GetComponentVelocity` (`self.Marble`))))
  (bind (_returnvalue_x_2 _returnvalue_y_2) (`KismetMathLibrary.BreakVector` (`KismetMathLibrary.Normal` (`KismetMathLibrary.MakeVector` _returnvalue_x _returnvalue_y _returnvalue_z))))
  (:`Triggered`
    (bind _ismaxspeed (`self.IsMaxSpeed`))
    (if (not _ismaxspeed)
      (`PrimitiveComponent.AddForce` (`self.Marble`) (* (`KismetMathLibrary.NegateVector` (`KismetMathLibrary.MakeVector` _returnvalue_x_2 _returnvalue_y_2)) (`self.force`)) "None" false))
    (`PrimitiveComponent.AddForce` (`self.Marble`) (* (`SceneComponent.GetRightVector` (`self.Camera`)) (* ActionValue (`self.force`))) "None" false)))

(event `EnhancedInput|/Game/Input/Actions/PlayerActions/IA_Look`
  (params (ActionValue :type "Vector2D Structure") (ElapsedSeconds :type "Float (double-precision)") (TriggeredSeconds :type "Float (double-precision)") (InputAction :type "InputAction Object Reference" :default "/Game/Input/Actions/PlayerActions/IA_Look.IA_Look"))
  (:`Triggered`
    (`self.AddControllerYawInput` ActionValue_X)
    (`self.AddControllerPitchInput` ActionValue_Y)))

(event `CustomEvent`
  (params (DeltaSeconds :type "Float (single-precision)")))

(event `self.ReceiveTick`
  (params (DeltaSeconds :type "Float (single-precision)"))
  (bind _isgrounded (`self.IsGrounded`))
  (set `self.canJump` (and _isgrounded (not (`self.brakeActive`)))))

(event `EnhancedInput|/Game/Input/Actions/PlayerActions/IA_Jump`
  (params (ActionValue :type Boolean) (ElapsedSeconds :type "Float (double-precision)") (TriggeredSeconds :type "Float (double-precision)") (InputAction :type "InputAction Object Reference" :default "/Game/Input/Actions/PlayerActions/IA_Jump.IA_Jump"))
  (bind (_returnvalue_x _returnvalue_y) (`KismetMathLibrary.BreakVector` (`SceneComponent.GetComponentVelocity` (`self.Marble`))))
  (:`Started`
    (if (`self.canJump`)
      (set `self.canJump` false)
      (`PrimitiveComponent.SetPhysicsLinearVelocity` (`self.Marble`) (`KismetMathLibrary.MakeVector` _returnvalue_x _returnvalue_y) false "None")
      (`PrimitiveComponent.AddImpulse` (`self.Marble`) (`KismetMathLibrary.MakeVector` 0.0 0.0 (`self.jumpForce`)) "None" true))))

(event `EnhancedInput|/Game/Input/Actions/PlayerActions/Up_Down_Action`
  (params (ActionValue :type "Float (double-precision)") (ElapsedSeconds :type "Float (double-precision)") (TriggeredSeconds :type "Float (double-precision)") (InputAction :type "InputAction Object Reference" :default "/Game/Input/Actions/PlayerActions/Up_Down_Action.Up_Down_Action"))
  (bind (_returnvalue_x _returnvalue_y _returnvalue_z) (`KismetMathLibrary.BreakVector` (`SceneComponent.GetComponentVelocity` (`self.Marble`))))
  (bind (_returnvalue_x_2 _returnvalue_y_2) (`KismetMathLibrary.BreakVector` (`KismetMathLibrary.Normal` (`KismetMathLibrary.MakeVector` _returnvalue_x _returnvalue_y _returnvalue_z))))
  (:`Triggered`
    (bind _ismaxspeed (`self.IsMaxSpeed`))
    (if (not _ismaxspeed)
      (`PrimitiveComponent.AddForce` (`self.Marble`) (* (`KismetMathLibrary.NegateVector` (`KismetMathLibrary.MakeVector` _returnvalue_x_2 _returnvalue_y_2)) (`self.force`)) "None" false))
    (`PrimitiveComponent.AddForce` (`self.Marble`) (* (`SceneComponent.GetForwardVector` (`self.Camera`)) (* ActionValue (`self.force`))) "None" false)))

(event `EnhancedInput|/Game/Input/Actions/PlayerActions/Brake_Action`
  (params (ActionValue :type Boolean) (ElapsedSeconds :type "Float (double-precision)") (TriggeredSeconds :type "Float (double-precision)") (InputAction :type "InputAction Object Reference" :default "/Game/Input/Actions/PlayerActions/Brake_Action.Brake_Action"))
  (bind _marble (`self.Marble`))
  (:`Triggered`
    (bind _isgrounded (`self.IsGrounded`))
    (if _isgrounded
      (set `self.brakeActive` true)
      (bind _output_get (set `self.linearDamping` (+ (`PrimitiveComponent.GetLinearDamping` (`self.Marble`)) 0.3)))
      (`PrimitiveComponent.SetLinearDamping` _marble _output_get)
      (else
        (bind _output_get_2 (set `self.linearDamping` 0.01 :!label _label))
        (set `self.brakeActive` false)
        (`PrimitiveComponent.SetLinearDamping` _marble _output_get_2))))
  (:`Completed`
    (goto _label)))

(fn `IsGrounded`
  (returns (isGrounded :type Boolean))
  (bind _returnvalue (`KismetMathLibrary.GetUpVector` (struct)))
  (bind _returnvalue_2 (+ (`SceneComponent.K2_GetComponentLocation` (`self.Marble`)) (* (10.0 10.0 10.0) _returnvalue)))
  (bind (_outhit _returnvalue_3) (`KismetSystemLibrary.SphereTraceSingle` _returnvalue_2 (- _returnvalue_2 (* _returnvalue (`self.groundTraceDistance`))) 45.0 "TraceTypeQuery1" false (`|MakeArray` self :!type "Actor Object Reference")))
  (if _returnvalue_3
    (if (>= (`KismetMathLibrary.Dot_VectorVector` (`.ImpactNormal` (`GameplayStatics.BreakHitResult` _outhit)) (`KismetMathLibrary.GetUpVector` (struct))) (`self.minGroundDot`))
      (return true)
      (else
        (return false)))
    (else
      (return false))))

(fn `IsMaxSpeed`
  (returns (IsMaxSpeed :type Boolean))
  (bind _returnvalue (`PrimitiveComponent.GetPhysicsLinearVelocity` (`self.Marble`) "None"))
  (return (<= (`KismetMathLibrary.VSize` _returnvalue) (`self.maxSpeed`))))

(fn `UserConstructionScript`)
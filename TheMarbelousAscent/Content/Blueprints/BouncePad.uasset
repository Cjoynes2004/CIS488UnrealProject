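; BouncePad is a pad that launches the player's marble along the pad's up vector when a "player"-tagged actor overlaps it.
; The overlap overwrites the cached Player_Marble's physics velocity with a scaled up vector and plays a 2D sound.
; A Tick countdown gates CanBoost, giving a cooldown between bounces.
; A disconnected alternative that reflects the marble's velocity off the pad via an impulse never runs.
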(event `self.ReceiveBeginPlay`
  (bind _asplayer_marble (cast `/Game/Blueprints/Player_Marble` (`GameplayStatics.GetPlayerPawn` 0)))
  (set `self.PlayerMarble` _asplayer_marble))

(event `self.ReceiveActorBeginOverlap`
  (params (OtherActor :type "Actor Object Reference"))
  (bind _output_get (set `self.Other Actor` OtherActor))
  (if (`self.CanBoost`)
    (if (`self.ActorHasTag` _output_get "player")
      (`PrimitiveComponent.SetPhysicsLinearVelocity` (`/Game/Blueprints/Player_Marble.Marble` (`self.PlayerMarble`)) (* (`SceneComponent.GetUpVector` (`self.BouncePad`)) (`self.BounceAmount`)) false "None")
      (set `self.CanBoost` false)
      (set `self.BounceWait` (`self.BounceMaxWait`))
      (`GameplayStatics.PlaySound2D` "/Game/Sounds/SFX/Shrinking/shrinking_sfx_landing.shrinking_sfx_landing" 1.0 1.0 0.0 null null))))

(event `self.ReceiveTick`
  (params (DeltaSeconds :type "Float (single-precision)"))
  (bind _output_get (set `self.BounceWait` (- (`self.BounceWait`) DeltaSeconds)))
  (if (<= _output_get 0.0)
    (set `self.CanBoost` true)
    (else
      (set `self.CanBoost` false))))

(fn `UserConstructionScript`)